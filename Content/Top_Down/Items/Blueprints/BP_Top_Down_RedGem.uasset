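; Red gem goal actor for top-down levels that completes the level when the player pawn hits it.
; Any hit destroys the gem, but only a player hit sets an unlock flag in gmInstance, indexed by the number parsed from the level name, and saves.
; It then removes the HUD, clears the touch interface, shows the Top_Down_LevelComplete widget and pauses the game.
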(event Collision|EventHit
  (params (MyComp :type Primitive%20Component%20Object%20Reference) (Other :type Actor%20Object%20Reference) (OtherComp :type Primitive%20Component%20Object%20Reference) (bSelfMoved :type Boolean) (HitLocation :type Vector :default "0, 0, 0") (HitNormal :type Vector :default "0, 0, 0") (NormalImpulse :type Vector :default "0, 0, 0") (Hit :type Hit%20Result%20Structure%20%28by%20ref%29))
  (Actor|DestroyActor)
  (if (== Other (Game|Player|GetPlayerPawn 0))
    (bind _returnvalue (Game|GetCurrentLevelName true))
    (bind _asgm_instance (Utilities|Casting|CastTogmInstance (Game|GetGameInstance)))
    (Development|PrintString (Utilities|String|RightChop _returnvalue 14))
    (Utilities|Array|SetArrayElem (Variables|/Game/gmInstance.gmInstance_C|GetGmInst_Top_Down_Level_Unlocked _asgm_instance) (Math|Conversions|ToInteger(Byte) (Utilities|String|RightChop _returnvalue 14)) true true)
    (Default|SaveGame _asgm_instance)
    (bind _asm_2d_player (Utilities|Casting|CastToM_2D_Player (Game|GetPlayerCharacter 0))
      (:then
        (Widget|RemovefromParent (Variables|/Game/M_2D_Player.M_2D_Player_C|GetHUD_Ref _asm_2d_player))
        (Class|PlayerController|ActivateTouchInterface (Game|GetPlayerController 0))
        (bind _returnvalue_2 (UserInterface|CreateWidget "/Game/Top_Down/UI/Top_Down_LevelComplete.Top_Down_LevelComplete_C" (Game|GetPlayerController 0)))
        (UserInterface|Viewport|AddtoViewport _returnvalue_2 0)
        (Game|SetGamePaused true)
        (Input|SetInputModeGameandUI (Game|GetPlayerController 0) _returnvalue_2 "DoNotLock" false))
      (:CastFailed
        (Development|PrintString "fail")))))

(fn ConstructionScript)