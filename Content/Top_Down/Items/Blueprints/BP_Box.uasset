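; BP_Box is a top-down box that the 2D player character (M_2D_Player) pushes by bumping into it.
; When the player hits the Box component, the sign of the hit normal's X, then Y, picks one axis for a small step.
; The step accumulates in NewVar0, which MoveComponentTo uses as the target relative location, with the rotation target held at a fixed pitch.
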(event OnComponentHit(Box)
  (params (HitComponent :type Primitive%20Component%20Object%20Reference) (OtherActor :type Actor%20Object%20Reference) (OtherComp :type Primitive%20Component%20Object%20Reference) (NormalImpulse :type Vector) (Hit :type Hit%20Result%20Structure%20%28by%20ref%29))
  (Utilities|Casting|CastToM_2D_Player OtherActor)
  (if (> (.x (.normal Hit)) 0.0)
    (Variables|Default|SetNewVar_0 (+ (Variables|Default|GetNewVar_0) "2.000000, 0, 0"))
    (Components|MoveComponentTo (Variables|Default|GetBox) (Variables|Default|GetNewVar_0) "0, 0,-90.000000" false false 0.2 false :!label _label)
    (elif (< (.x (.normal Hit)) 0.0)
      (Variables|Default|SetNewVar_0 (+ (Variables|Default|GetNewVar_0) "-2.000000, 0, 0"))
      (goto _label)
      (elif (> (.y (.normal Hit)) 0.0)
        (Variables|Default|SetNewVar_0 (+ (Variables|Default|GetNewVar_0) "0.000000,2.000000, 0"))
        (goto _label)
        (elif (< (.y (.normal Hit)) 0.0)
          (Variables|Default|SetNewVar_0 (+ (Variables|Default|GetNewVar_0) "0.000000,-2.000000, 0"))
          (goto _label))))))

(event EventBeginPlay)

(event Collision|EventActorBeginOverlap
  (params (OtherActor :type Actor%20Object%20Reference)))

(event EventTick
  (params (DeltaSeconds :type Float%20%28single-precision%29)))

(fn ConstructionScript)