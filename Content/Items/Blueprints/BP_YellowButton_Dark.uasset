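; BP_YellowButton_Dark is a sprite-based yellow button that the player presses on hit, but only while it is pressable.
; A linked switch's OnFlip toggles pressability and swaps between lit and dark sprites.
; A press changes the sprite, broadcasts YellowBtnPressedNOPWR and optionally plays a Matinee.
; A timer then calls Reset, which restores the lit sprite, broadcasts the release and optionally plays the Matinee again.
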(event Custom|CustomEvent_0
  (if (Variables|Default|GetPressable)
    (Variables|Default|SetPressable false)
    (Rendering|Components|Sprite|SetSprite (Variables|Default|GetPaperSprite) "/Game/Items/Sprites/YellowButtonDark.YellowButtonDark")
    (else
      (Variables|Default|SetPressable true)
      (Rendering|Components|Sprite|SetSprite (Variables|Default|GetPaperSprite) "/Game/Items/Sprites/YellowButton.YellowButton"))))

(event EventBeginPlay
  (if (Variables|Default|GetPressable)
    (Rendering|Components|Sprite|SetSprite (Variables|Default|GetPaperSprite) "/Game/Items/Sprites/YellowButton.YellowButton")
    (else
      (Rendering|Components|Sprite|SetSprite (Variables|Default|GetPaperSprite) "/Game/Items/Sprites/YellowButtonDark.YellowButtonDark")))
  (EventDispatchers|BindEventtoOnFlip (Variables|Default|Getswitch_ref) (delegate Custom|CustomEvent_0)))

(event Collision|EventHit
  (params (MyComp :type Primitive%20Component%20Object%20Reference) (Other :type Actor%20Object%20Reference) (OtherComp :type Primitive%20Component%20Object%20Reference) (bSelfMoved :type Boolean) (HitLocation :type Vector :default "0, 0, 0") (HitNormal :type Vector :default "0, 0, 0") (NormalImpulse :type Vector :default "0, 0, 0") (Hit :type Hit%20Result%20Structure%20%28by%20ref%29))
  (if (and (== Other (Game|Player|GetPlayerPawn 0)) (Variables|Default|GetPressable))
    (Rendering|Components|Sprite|SetSprite (Variables|Default|GetPaperSprite) "/Game/Items/Sprites/YellowButtonPressed.YellowButtonPressed")
    (bind _output_get (Variables|Default|Setpressed true))
    (Default|CallYellowBtnPressedNOPWR _output_get)
    (if (Variables|Default|GetPlayAnimation)
      (Audio|Components|Audio|Play (Variables|Default|GetMatineeRef)))
    (Utilities|Time|SetTimerbyFunctionName 0 "Reset" (Variables|Default|GetTime))))

(fn ConstructionScript)

(fn Reset
  (Rendering|Components|Sprite|SetSprite (Variables|Default|GetPaperSprite) "/Game/Items/Sprites/YellowButton.YellowButton")
  (Variables|Default|Setpressed false)
  (Default|CallYellowBtnPressedNOPWR false)
  (if (Variables|Default|GetPlayAnimation)
    (Audio|Components|Audio|Play (Variables|Default|GetMatineeRef))))