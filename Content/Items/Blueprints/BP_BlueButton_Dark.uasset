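; BP_BlueButton_Dark is a blue sprite button that the player pawn hits to move a wall or play a Matinee.
; A hit only works while Pressable is set, swapping to the pressed sprite and, depending on UseBP, activating the wall's InterpToMovement or playing MatineeRef.
; A linked switch's OnFlip event toggles Pressable, swapping between the normal and dark sprites.
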(event Custom|CustomEvent_0
  (if (Variables|Default|GetPressable)
    (Variables|Default|SetPressable false)
    (Rendering|Components|Sprite|SetSprite (Variables|Default|GetPaperSprite) "/Game/Items/Sprites/BlueButtonDark.BlueButtonDark")
    (else
      (Variables|Default|SetPressable true)
      (Rendering|Components|Sprite|SetSprite (Variables|Default|GetPaperSprite) "/Game/Items/Sprites/BlueButton.BlueButton"))))

(event EventBeginPlay
  (if (Variables|Default|GetPressable)
    (Rendering|Components|Sprite|SetSprite (Variables|Default|GetPaperSprite) "/Game/Items/Sprites/BlueButton.BlueButton")
    (else
      (Rendering|Components|Sprite|SetSprite (Variables|Default|GetPaperSprite) "/Game/Items/Sprites/BlueButtonDark.BlueButtonDark")))
  (EventDispatchers|BindEventtoOnFlip (Variables|Default|Getswitch_ref) (delegate Custom|CustomEvent_0)))

(event Collision|EventHit
  (params (MyComp :type Primitive%20Component%20Object%20Reference) (Other :type Actor%20Object%20Reference) (OtherComp :type Primitive%20Component%20Object%20Reference) (bSelfMoved :type Boolean) (HitLocation :type Vector :default "0, 0, 0") (HitNormal :type Vector :default "0, 0, 0") (NormalImpulse :type Vector :default "0, 0, 0") (Hit :type Hit%20Result%20Structure%20%28by%20ref%29))
  (if (and (== Other (Game|Player|GetPlayerPawn 0)) (Variables|Default|GetPressable))
    (Rendering|Components|Sprite|SetSprite (Variables|Default|GetPaperSprite) "/Game/Items/Sprites/BlueButtonPressed.BlueButtonPressed")
    (if (Variables|Default|GetUse%20BP)
      (Components|Activation|Activate (Variables|/Game/Items/Blueprints/BP_Wall.BP_Wall_C|GetInterpToMovement (Variables|Default|GetWall)) false)
      (else
        (Audio|Components|Audio|Play (Variables|Default|GetMatineeRef))))))

(fn ConstructionScript)