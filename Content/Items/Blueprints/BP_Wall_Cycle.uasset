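; BP_Wall_Cycle is a wall that runs a down-and-back-up movement cycle, with a pause before rising.
; BeginPlay sets distance and speed, and Tick drives a Direction state machine that builds a spline for each leg and follows it until finished.
; Finishing the descent flips Direction to rise after a Delay; finishing the rise updates Position and idles at Direction zero, with nothing here restarting it.
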(event EventBeginPlay
  (Variables|Default|SetDistance 2e+01)
  (Variables|Default|SetSpeed 0.4))

(event Collision|EventActorBeginOverlap
  (params (OtherActor :type Actor%20Object%20Reference)))

(event EventTick
  (params (DeltaSeconds :type Float%20%28single-precision%29))
  (if (== (Variables|Default|GetDirection) -1)
    (if (Variables|Default|GetSplineMade)
      (Variables|Default|SetFollow true)
      (bind _completed (CallFunction|FollowSpline))
      (if _completed
        (Variables|Default|SetDirection 1)
        (Variables|Default|SetSplineMade false)
        (Variables|Default|SetFollow false)
        (Variables|Default|SetSplineDistance 0.0)
        (Variables|Default|SetPosition "NewEnumerator1"))
      (else
        (bind _splinemade (CallFunction|MakeSplineDown))
        (Variables|Default|SetSplineMade _splinemade)))
    (elif (== (Variables|Default|GetDirection) 1)
      (if (Variables|Default|GetHasWaited)
        (if (Variables|Default|GetSplineMade)
          (Variables|Default|SetFollow true)
          (bind _completed_2 (CallFunction|FollowSpline))
          (if _completed_2
            (Variables|Default|SetDirection 0)
            (Variables|Default|SetSplineMade false)
            (Variables|Default|SetFollow false)
            (Variables|Default|SetSplineDistance 0.0)
            (Variables|Default|SetPosition "NewEnumerator0")
            (Variables|Default|SetHasWaited false))
          (else
            (bind _splinemade_2 (CallFunction|MakeSplineUp))
            (Variables|Default|SetSplineMade _splinemade_2)))
        (else
          (Utilities|FlowControl|Delay (Variables|Default|GetDuration))
          (Variables|Default|SetHasWaited true))))))

(fn ConstructionScript)