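; BP_RedButton is a Paper2D red button that toggles a referenced Matinee sequence when hit.
; A hit from the player pawn shows the pressed sprite, and a timer calls Reset to restore it.
; Any hit also advances a FlipFlop that alternately plays or reverses the Matinee, guarded by a Played flag that updates after a delay sharing the timer's duration.
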(event Collision|EventHit
  (params (MyComp :type Primitive%20Component%20Object%20Reference) (Other :type Actor%20Object%20Reference) (OtherComp :type Primitive%20Component%20Object%20Reference) (bSelfMoved :type Boolean) (HitLocation :type Vector :default "0, 0, 0") (HitNormal :type Vector :default "0, 0, 0") (NormalImpulse :type Vector :default "0, 0, 0") (Hit :type Hit%20Result%20Structure%20%28by%20ref%29))
  (bind _matineeref (Variables|Default|GetMatineeRef))
  (bind _time (Variables|Default|GetTime))
  (Utilities|FlowControl|Sequence
    (:then_0
      (if (== Other (Game|Player|GetPlayerPawn 0))
        (Rendering|Components|Sprite|SetSprite (Variables|Default|GetPaperSprite) "/Game/Items/Sprites/RedButtonPressed.RedButtonPressed")
        (Utilities|Time|SetTimerbyFunctionName 0 "Reset" (Variables|Default|GetTime))))
    (:then_1
      (Utilities|FlowControl|FlipFlop
        (:A
          (if (not (Variables|Default|GetPlayed))
            (Audio|Components|Audio|Play _matineeref)
            (Utilities|FlowControl|Delay _time)
            (Variables|Default|SetPlayed true)))
        (:B
          (if (Variables|Default|GetPlayed)
            (Utilities|String|Reverse _matineeref)
            (Utilities|FlowControl|Delay _time)
            (Variables|Default|SetPlayed false)))))))

(fn ConstructionScript)

(fn Reset
  (Rendering|Components|Sprite|SetSprite (Variables|Default|GetPaperSprite) "/Game/Items/Sprites/RedButton.RedButton"))