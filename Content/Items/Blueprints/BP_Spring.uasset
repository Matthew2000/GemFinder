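; BP_Spring is a spring pad that launches the player character when their pawn overlaps its box trigger.
; On overlap it swaps the paper sprite to the extended spring, applies the Distance vector as a launch velocity and sets Pressed.
; A timer of configurable Time then calls a reset function that restores the lowered sprite and clears Pressed.
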(event OnComponentBeginOverlap(Box)
  (params (OverlappedComponent :type Primitive%20Component%20Object%20Reference) (OtherActor :type Actor%20Object%20Reference) (OtherComp :type Primitive%20Component%20Object%20Reference) (OtherBodyIndex :type Integer) (bFromSweep :type Boolean) (SweepResult :type Hit%20Result%20Structure%20%28by%20ref%29))
  (if (== OtherActor (Game|Player|GetPlayerPawn 0))
    (Rendering|Components|Sprite|SetSprite (Variables|Default|GetPaperSprite) "/Game/Items/Sprites/Spring_Up.Spring_Up")
    (Character|LaunchCharacter (Game|GetPlayerCharacter 0) (Variables|Default|GetDistance) false false)
    (Variables|Default|SetPressed true)
    (Utilities|Time|SetTimerbyFunctionName 0 "reset Spring" (Variables|Default|GetTime))))

(fn ConstructionScript)

(fn ResetSpring
  (Rendering|Components|Sprite|SetSprite (Variables|Default|GetPaperSprite) "/Game/Items/Sprites/Spring_Down.Spring_Down")
  (Variables|Default|SetPressed false))