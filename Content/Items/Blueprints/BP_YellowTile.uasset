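; BP_YellowTile is a tile whose collision follows the pressed state of a linked yellow button.
; UseDarkButton selects whether it binds to the dark button's NOPWR event or the regular button's PWR event.
; Both handlers enable query and physics collision when pressed and disable collision otherwise.
; The binding is made on every Tick rather than once at BeginPlay.
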(event Custom|CustomEvent_0
  (params (Pressed :type Boolean))
  (if Pressed
    (Collision|SetCollisionEnabled (Variables|Default|GetYellowTile) "QueryAndPhysics")
    (else
      (Collision|SetCollisionEnabled (Variables|Default|GetYellowTile) "NoCollision"))))

(event Custom|CustomEvent_1
  (params (Pressed :type Boolean))
  (if Pressed
    (Collision|SetCollisionEnabled (Variables|Default|GetYellowTile) "QueryAndPhysics")
    (else
      (Collision|SetCollisionEnabled (Variables|Default|GetYellowTile) "NoCollision"))))

(event EventTick
  (params (DeltaSeconds :type Float%20%28single-precision%29))
  (if (Variables|Default|GetUseDarkButton)
    (EventDispatchers|BindEventtoYellowBtnPressedNOPWR (Variables|Default|GetYellowBtnDarkRef) (delegate Custom|CustomEvent_1))
    (else
      (EventDispatchers|BindEventtoYellowBtnPressedPWR (Variables|Default|GetYellowBtnRef) (delegate Custom|CustomEvent_0)))))

(fn ConstructionScript)