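; A 2D side-scroller switch that the player flips with the HUD's activate button while overlapping its box.
; Tick polls the button and consumes the HUD's Flip flag to limit repeat triggers, then alternates the up and down sprites.
; Each flip calls OnFlip and starts every actor in the Wall array following, with direction chosen from that wall's current Position.
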(event EventTick
  (params (DeltaSeconds :type Float%20%28single-precision%29))
  (bind _as2dside_scroller_character (Utilities|Casting|CastTo2DSideScrollerCharacter (Game|GetPlayerCharacter 0)))
  (bind _output_get (Variables|Default|SetHUDref (Variables|/Game/2DSideScrollerBP/Blueprints/2DSideScrollerCharacter.2DSideScrollerCharacter_C|GetHUD%20reference _as2dside_scroller_character)))
  (if (and (Class|Button|IsPressed (Variables|/Game/UI/HUD.HUD_C|GetActivateButton _output_get)) (Collision|IsOverlappingActor (Variables|Default|GetBox) (Game|Player|GetPlayerPawn 0) :!class /Script/Engine.PrimitiveComponent))
    (if (Variables|/Game/UI/HUD.HUD_C|Getflip (Variables|Default|GetHUDref))
      (Variables|/Game/UI/HUD.HUD_C|Setflip (Variables|Default|GetHUDref) false)
      (Utilities|FlowControl|FlipFlop
        (:A
          (Rendering|Components|Sprite|SetSprite (Variables|Default|GetPaperSprite) "/Game/Items/Sprites/SwitchDown.SwitchDown"))
        (:B
          (Rendering|Components|Sprite|SetSprite (Variables|Default|GetPaperSprite) "/Game/Items/Sprites/SwitchUp.SwitchUp")))
      (Default|CallOnFlip)
      (Utilities|FlowControl|Sequence
        (:then_0
          (for _array_element (Variables|Default|GetWall)
            (if (Utilities|Enum|Equal(Enum) (Variables|/Game/Items/Blueprints/BP_Wall.BP_Wall_C|GetPosition _array_element) "NewEnumerator0")
              (Variables|/Game/Items/Blueprints/BP_Wall.BP_Wall_C|SetDirection _array_element -1)
              (Variables|/Game/Items/Blueprints/BP_Wall.BP_Wall_C|SetFollow _array_element true)
              (else
                (Variables|/Game/Items/Blueprints/BP_Wall.BP_Wall_C|SetDirection _array_element 1)
                (Variables|/Game/Items/Blueprints/BP_Wall.BP_Wall_C|SetFollow _array_element true)))))))))

(fn ConstructionScript)